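; Game mode for a bow and arrow game on an nDisplay cluster that keeps three point tiers of targets populated around the players.
; Each tick the master tops up tier counts with random ring positions, spacing-checked against existing targets, encoded as string map entries.
; A cluster event broadcasts that map so nodes spawn matching center-facing targets, with a direct call in editor.
; DestroyTarget removes targets and lowers counts, triggering replacements.
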(event EventBeginPlay
  (Utilities|FlowControl|Sequence
    (:then_0
      ;[1 1 1] Listen to our own cluster events
      (Class|DisplayClusterBlueprintAPI|AddClusterEventListener (Class|DisplayClusterBlueprintLib|GetAPI) self))))

(event EventTick
  (params (DeltaSeconds :type Float%20%28single-precision%29))
  (bind _returnvalue (CallFunction|IsEditor))
  (bind _returnvalue_2 (Class|DisplayClusterBlueprintAPI|IsMaster (Class|DisplayClusterBlueprintLib|GetAPI)))
  (if (or _returnvalue_2 _returnvalue)
    (CallFunction|CreateNewTargetsMaster)))

(event EventOnClusterEvent
  (params (Event :type Display%20Cluster%20Cluster%20Event%20Structure%20%28by%20ref%29))
  (bind (_name _type _category _parameters) (Utilities|Struct|BreakDisplayClusterClusterEvent Event))
  (switch string _name
    (:CreateNewTargets
      (CallFunction|CreateNewTargets _parameters))))

(fn ConstructionScript)

(fn CreateNewTargets
  (params (Instructions :type Map%20of%20Strings%20to%20Strings))
  (bind _keys (Utilities|Map|Keys Instructions))
  (for _array_element _keys
    (bind _returnvalue (Game|SpawnActorfromClass "/Game/BowArrow/Target.Target_C" (Math|Transform|MakeTransform (Math|Vector|MakeVector (Math|Conversions|ToFloat(Integer) (Utilities|Array|Get(acopy) (Utilities|String|ParseIntoArray _array_element "_"))) (Math|Conversions|ToFloat(Integer) (Utilities|Array|Get(acopy) (Utilities|String|ParseIntoArray _array_element "_") 1)) (Math|Conversions|ToFloat(Integer) (Utilities|Array|Get(acopy) (Utilities|String|ParseIntoArray _array_element "_") 2))) (Math|Conversions|RotationFromXVector (* (Math|Vector|MakeVector (Math|Conversions|ToFloat(Integer) (Utilities|Array|Get(acopy) (Utilities|String|ParseIntoArray _array_element "_"))) (Math|Conversions|ToFloat(Integer) (Utilities|Array|Get(acopy) (Utilities|String|ParseIntoArray _array_element "_") 1)) 0.0) -1.0))) "Undefined" 0 0))
    (switch int (Math|Conversions|ToInteger(Byte) (.Value (Utilities|Map|Find Instructions _array_element)))
      (:Default
        (Default|SetPointValue _returnvalue 1 :!label _label)
        (Utilities|Array|Add (Variables|Default|GetTargetsLow) _returnvalue))
      (:0
        (goto _label))
      (:1
        (Default|SetPointValue _returnvalue 2)
        (Utilities|Array|Add (Variables|Default|GetTargetsMid) _returnvalue))
      (:2
        (Default|SetPointValue _returnvalue 5)
        (Utilities|Array|Add (Variables|Default|GetTargetsHigh) _returnvalue)))))

(fn CreateNewTargetsMaster
  (bind _targetstocreate (LocalVariables|GettargetsToCreate))
  (Utilities|FlowControl|Sequence
    (:then_0
      ;[1 1 1] Generate instructions for each target that needs to be created. Each map element as follows: [xPos_yPos_zPos], [type] (where type is index of low/mid/high, i.e. 0/1/2)
      (while (< (Variables|Default|GettargetsLowCurrent) (Variables|Default|GettargetsLowMax))
        (bind (_positionx _positiony _positionz) (CallFunction|GetRandomTargetPosition 3.5e+02 7.5e+02 1e+03))
        (Utilities|Map|Add (LocalVariables|GettargetsToCreate) (Utilities|String|Append _positionx "_" _positiony "_" _positionz) "0")
        (Math|Integer|IncrementInt (Variables|Default|GettargetsLowCurrent))))
    (:then_1
      (while (< (Variables|Default|GettargetsMidCurrent) (Variables|Default|GettargetsMidMax))
        (bind (_positionx_2 _positiony_2 _positionz_2) (CallFunction|GetRandomTargetPosition 3.5e+02 1.5e+03 1.75e+03))
        (Utilities|Map|Add (LocalVariables|GettargetsToCreate) (Utilities|String|Append _positionx_2 "_" _positiony_2 "_" _positionz_2) "1")
        (Math|Integer|IncrementInt (Variables|Default|GettargetsMidCurrent))))
    (:then_2
      (while (< (Variables|Default|GettargetsHighCurrent) (Variables|Default|GettargetsHighMax))
        (bind (_positionx_3 _positiony_3 _positionz_3) (CallFunction|GetRandomTargetPosition 3.5e+02 1.1e+03 1.4e+03))
        (Utilities|Map|Add (LocalVariables|GettargetsToCreate) (Utilities|String|Append _positionx_3 "_" _positiony_3 "_" _positionz_3) "2")
        (Math|Integer|IncrementInt (Variables|Default|GettargetsHighCurrent))))
    (:then_3
      (if (> (Utilities|Map|Length _targetstocreate) 0)
        (bind _returnvalue (CallFunction|IsEditor))
        (if _returnvalue
          (CallFunction|CreateNewTargets _targetstocreate)
          (else
            (Class|DisplayClusterBlueprintAPI|EmitClusterEvent (Class|DisplayClusterBlueprintLib|GetAPI) (Utilities|Struct|MakeDisplayClusterClusterEvent "CreateNewTargets" "" "" _targetstocreate) false)))))))

(fn GetRandomTargetPosition
  (params (height :type Float%20%28single-precision%29) (minDistance :type Float%20%28single-precision%29) (maxDistance :type Float%20%28single-precision%29))
  (bind _returnvalue (- height 75.0))
  (bind _returnvalue_2 (- maxDistance minDistance))
  (bind _returnvalue_3 (Math|Random|RandomFloat))
  (bind _returnvalue_4 (Math|Random|RandomFloat))
  (bind _returnvalue_5 (Math|Random|RandomFloat))
  (bind _returnvalue_6 (* _returnvalue_5 _returnvalue_2))
  (bind _returnvalue_7 (* _returnvalue_3 _returnvalue))
  (bind _returnvalue_8 (* _returnvalue_4 3.6e+02))
  (bind _returnvalue_9 (Math|Trig|Cos(Degrees) _returnvalue_8))
  (bind _returnvalue_10 (Math|Trig|Sin(Degrees) _returnvalue_8))
  (bind _returnvalue_11 (+ minDistance _returnvalue_6))
  (bind _returnvalue_12 (+ _returnvalue_7 75.0))
  (bind _returnvalue_13 (* _returnvalue_10 _returnvalue_11))
  (bind _returnvalue_14 (* _returnvalue_9 _returnvalue_11))
  (while (not (LocalVariables|GetfoundValidPos))
    (bind _isvalid (CallFunction|IsTargetPositionValid (Math|Vector|MakeVector _returnvalue_14 _returnvalue_13 _returnvalue_12)))
    (if _isvalid
      (return (Utilities|String|ToString(Float) _returnvalue_14) (Utilities|String|ToString(Float) _returnvalue_13) (Utilities|String|ToString(Float) _returnvalue_12))
      (else
        (Math|Integer|IncrementInt (LocalVariables|GetcurrentCount)
          (:%20%20
            (if (>= (LocalVariables|GetcurrentCount) (LocalVariables|GetmaxCount))
              (LocalVariables|SetfoundValidPos true)))))))
  (return "0" "0" "-500"))

(fn IsTargetPositionValid
  (params (targetPosition :type Vector))
  (Utilities|FlowControl|Sequence
    (:then_0
      (for _array_element (Variables|Default|GetTargetsLow)
        (if (<= (Math|Vector|Distance(Vector) (Transformation|GetActorLocation _array_element) targetPosition) (Variables|Default|GetminSpaceBetweenTargets))
          (return false))))
    (:then_1
      (for _array_element_2 (Variables|Default|GetTargetsMid)
        (if (<= (Math|Vector|Distance(Vector) (Transformation|GetActorLocation _array_element_2) targetPosition) (Variables|Default|GetminSpaceBetweenTargets))
          (return false))))
    (:then_2
      (for _array_element_3 (Variables|Default|GetTargetsHigh)
        (if (<= (Math|Vector|Distance(Vector) (Transformation|GetActorLocation _array_element_3) targetPosition) (Variables|Default|GetminSpaceBetweenTargets))
          (return false))))
    (:then_3
      (return true))))

(fn DestroyTarget
  (params (bowArrowTarget :type Target%20Object%20Reference))
  (switch int (Variables|/Game/BowArrow/Target.Target_C|GetpointValue bowArrowTarget)
    (:Default
      (Math|Integer|DecrementInt (Variables|Default|GettargetsHighCurrent) :!label _label
        (:%20%20
          (Utilities|Array|RemoveItem (Variables|Default|GetTargetsHigh) bowArrowTarget))))
    (:0
      (Math|Integer|DecrementInt (Variables|Default|GettargetsLowCurrent) :!label _label_2
        (:%20%20
          (Utilities|Array|RemoveItem (Variables|Default|GetTargetsLow) bowArrowTarget))))
    (:1
      (goto _label_2))
    (:2
      (Math|Integer|DecrementInt (Variables|Default|GettargetsMidCurrent)
        (:%20%20
          (Utilities|Array|RemoveItem (Variables|Default|GetTargetsMid) bowArrowTarget))))
    (:3
      (goto _label)))
  (Actor|DestroyActor bowArrowTarget))

(fn IsEditor
  ;[1 1 1] Allows code to run when testing in editor
  (bind _returnvalue (Class|DisplayClusterBlueprintAPI|GetAllNodes (Class|DisplayClusterBlueprintLib|GetAPI)))
  (return (<= (Utilities|Array|Length _returnvalue) 0)))