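; Quokka Conundrum actor that acts as either a tracker-driven elevator or rotator, chosen by IsElevator, hiding the unused mesh and disabling its collision.
; Before GameStarted, the elevator continually records the tracker's DA-space Y as StartingHeight.
; Once started, it shifts along world Y each tick by tracker Y plus StartingHeight, scaled by MoveSpeed without delta time.
; The rotator instead copies the tracker's relative pitch.
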(event EventBeginPlay
  (|CallParentFunction)
  (if (Variables|Default|GetIsElevator)
    (CallFunction|DisableMesh (Variables|Default|GetRotatorMesh))
    (else
      (CallFunction|DisableMesh (Variables|Default|GetElevatorMesh)))))

(event Collision|EventActorBeginOverlap
  (params (OtherActor :type Actor%20Object%20Reference))
  (|CallParentFunction OtherActor) ; This node is disabled and will not be called.\nDrag off pins to build functionality.
)

(event EventTick
  (params (DeltaSeconds :type Float%20%28single-precision%29))
  (|CallParentFunction DeltaSeconds)
  (if (Variables|Default|GetGameStarted)
    (if (Variables|Default|GetIsElevator)
      (CallFunction|MoveElevator)
      (else
        (CallFunction|MoveRotator)))
    (elif (Variables|Default|GetIsElevator)
      (CallFunction|CalibrateElevator))))

(fn ConstructionScript
  (|CallParentFunction))

(fn DisableMesh
  (params (MeshToDisable :type Static%20Mesh%20Component%20Object%20Reference))
  (Development|SetHiddeninGame MeshToDisable true false)
  (Collision|SetCollisionEnabled MeshToDisable "NoCollision"))

(fn MoveElevator
  (bind _returnvalue (Transformation|GetActorLocation))
  (bind (_x _y _z) (Math|Vector|BreakVector _returnvalue))
  ;[1 1 1] Get DA Tracker and Determine distance based on prior calibration
  (bind _datracker (CallFunction|GetTrackerasDATracker "NewEnumerator0"))
  (bind _location (Default|GetLocationinDA _datracker))
  ;[1 1 1] Move the Actor based on maths
  (Transformation|SetActorLocation (Math|Vector|MakeVector _x (+ (* (+ (.Y (Math|Vector|BreakVector _location)) (Variables|Default|GetStartingHeight)) (Variables|Default|GetMoveSpeed)) _y) _z) false false))

(fn MoveRotator
  (bind _returnvalue (Transformation|GetActorRotation))
  (bind (_roll _pitch _yaw) (Math|Rotator|BreakRotator _returnvalue))
  ;[1 1 1] Get DA Tracker Rotation and create Rotator, then rotate Actor
  (bind _datracker (CallFunction|GetTrackerasDATracker "NewEnumerator0"))
  (bind _rotation (Default|GetRelativeRotation _datracker))
  (Transformation|SetActorRotation (Math|Rotator|MakeRotator _roll (.Pitch (Math|Rotator|BreakRotator _rotation)) _yaw)))

(fn CalibrateElevator
  ;[1 1 1] Set the starting height to whatever the current height of the tracker is
  (bind _datracker (CallFunction|GetTrackerasDATracker "NewEnumerator0"))
  (bind _location (Default|GetLocationinDA _datracker))
  (Variables|Default|SetStartingHeight (.Y (Math|Vector|BreakVector _location))))