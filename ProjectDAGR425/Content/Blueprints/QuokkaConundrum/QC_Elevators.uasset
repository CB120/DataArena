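; QC_Elevators is a Quokka Conundrum Blueprint with helper functions for elevators driven by left and right tracker positions.
; CalibrateTrackers stores both trackers' current locations as start positions.
; MoveElevatorL returns the sum of the left start position and current left tracker location, without moving anything itself.
; The event graph is inactive, nothing here calls either function, and the right side has no move function.
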(event EventBeginPlay
  (|CallParentFunction) ; This node is disabled and will not be called.\nDrag off pins to build functionality.
)

(event Collision|EventActorBeginOverlap
  (params (OtherActor :type Actor%20Object%20Reference))
  (|CallParentFunction OtherActor) ; This node is disabled and will not be called.\nDrag off pins to build functionality.
)

(event EventTick
  (params (DeltaSeconds :type Float%20%28single-precision%29))
  (|CallParentFunction DeltaSeconds) ; This node is disabled and will not be called.\nDrag off pins to build functionality.
)

(fn ConstructionScript
  (|CallParentFunction))

(fn CalibrateTrackers
  (bind _location (CallFunction|GetTrackerLocation "NewEnumerator1"))
  (Variables|Default|SetStartPosL _location)
  (bind _location_2 (CallFunction|GetTrackerLocation "NewEnumerator0"))
  (Variables|Default|SetStartPosR _location_2))

(fn MoveElevatorL
  (bind _location (CallFunction|GetTrackerLocation "NewEnumerator1"))
  (return (+ (Variables|Default|GetStartPosL) _location)))