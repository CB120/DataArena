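; ElevatorManager is an actor that coordinates the left and right tracker-driven elevators in the Quokka Conundrum game.
; AssignDATrackers stores both elevator references and hands each a DATracker, printing an error if a cast fails.
; While GameStarted is true, Tick moves both elevators every frame through MoveElevators.
; CalibrateElevators forwards calibration to the left elevator only.
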(event EventBeginPlay
  (|CallParentFunction) ; This node is disabled and will not be called.\nDrag off pins to build functionality.
)

(event Collision|EventActorBeginOverlap
  (params (OtherActor :type Actor%20Object%20Reference))
  (|CallParentFunction OtherActor) ; This node is disabled and will not be called.\nDrag off pins to build functionality.
)

(event EventTick
  (params (DeltaSeconds :type Float%20%28single-precision%29))
  (|CallParentFunction DeltaSeconds)
  (if (Variables|Default|GetGameStarted)
    (CallFunction|MoveElevators)))

(fn ConstructionScript
  (|CallParentFunction))

(fn AssignDATrackers
  (params (ElevatorL :type Elevator%20Object%20Reference) (ElevatorR :type Elevator%20Object%20Reference))
  ;[1 1 1] Assign Elevator References
  (bind _output_get (Variables|Default|SetElevatorL ElevatorL))
  (bind _output_get_2 (Variables|Default|SetElevatorR ElevatorR))
  ;[1 1 1] Assign the Left Tracker
  (bind (_datracker _castsucceeded) (CallFunction|GetTrackerasDATracker "NewEnumerator1"))
  (if _castsucceeded
    (Default|AssignDATracker _output_get _datracker)
    ;[1 1 1] Assign the Right Tracker
    (bind (_datracker_2 _castsucceeded_2) (CallFunction|GetTrackerasDATracker "NewEnumerator0"))
    (if _castsucceeded_2
      (Default|AssignDATracker _output_get_2 _datracker_2)
      (else
        (Development|PrintString "Error: Couldn't Assign Right Tracker in ElevatorManager" true true "(R=1.000000,G=0.047278,B=0.000000,A=1.000000)")))
    (else
      (Development|PrintString "Error: Couldn't Assign Left Tracker in ElevatorManager" true true "(R=1.000000,G=0.047278,B=0.000000,A=1.000000)"))))

(fn MoveElevators
  (Default|MoveElevator (Variables|Default|GetElevatorL))
  (Default|MoveElevator (Variables|Default|GetElevatorR)))

(fn CalibrateElevators
  (Default|CalibrateElevator (Variables|Default|GetElevatorL)))