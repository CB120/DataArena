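; QC_Manager is the manager Blueprint that sets up player pairs for the Quokka Conundrum game.
; On BeginPlay it casts each entry in PlayerPairs to QC_Pair, flags even-indexed pairs as elevators, and moves each to the SpawnPoints and RelativeRotations entry at the same index.
; A failed cast prints an error, and the construction script only calls its parent.
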(event EventBeginPlay
  (|CallParentFunction)
  (Utilities|FlowControl|Sequence
    (:then_0
      (for (_array_element _array_index) (Variables|Default|GetplayerPairs)
        (bind _asqc_pair (Utilities|Casting|CastToQC_Pair _array_element)
          (:then
            (Variables|/Game/Blueprints/QuokkaConundrum/QC_Pair.QC_Pair_C|SetIsElevator _asqc_pair (== (Math|Integer|%(Integer) _array_index 2) 0))
            (Transformation|SetActorLocationAndRotation _asqc_pair (Utilities|Array|Get(acopy) (Variables|Default|GetSpawnPoints) _array_index) (Utilities|Array|Get(acopy) (Variables|Default|GetRelativeRotations) _array_index)))
          (:CastFailed
            (Development|PrintString "Error: Cast to QC_Pair Failed in QC_Manager BeginPlay" true true "(R=1.000000,G=0.000000,B=0.014251,A=1.000000)")))))))

(event Collision|EventActorBeginOverlap
  (params (OtherActor :type Actor%20Object%20Reference))
  (|CallParentFunction OtherActor) ; This node is disabled and will not be called.\nDrag off pins to build functionality.
)

(event EventTick
  (params (DeltaSeconds :type Float%20%28single-precision%29))
  (|CallParentFunction DeltaSeconds) ; This node is disabled and will not be called.\nDrag off pins to build functionality.
)

(fn ConstructionScript
  (|CallParentFunction))