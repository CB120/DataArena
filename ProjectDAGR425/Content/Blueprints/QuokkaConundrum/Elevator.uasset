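; Elevator actor for Quokka Conundrum that moves along its world Y axis, driven by the position of an externally assigned DATracker.
; CalibrateElevator stores the tracker's current DA-space Y as StartingHeight.
; Each MoveElevator call adds the tracker Y plus StartingHeight, scaled by MoveSpeed, to the actor's Y without sweep, so movement accumulates.
; BeginPlay and Tick are empty, so calibration and movement rely on external calls.
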(event EventBeginPlay)

(event EventTick
  (params (DeltaSeconds :type Float%20%28single-precision%29)))

(fn ConstructionScript)

(fn CalibrateElevator
  ;[1 1 1] Set the starting height to whatever the current height of the tracker is
  (bind _location (Default|GetLocationinDA (Variables|Default|GetDA_Tracker)))
  (Variables|Default|SetStartingHeight (.Y (Math|Vector|BreakVector _location))))

(fn MoveElevator
  (bind _returnvalue (Transformation|GetActorLocation))
  (bind (_x _y _z) (Math|Vector|BreakVector _returnvalue))
  ;[1 1 1] Get DA Tracker and Determine distance based on prior calibration
  (bind _location (Default|GetLocationinDA (Variables|Default|GetDA_Tracker)))
  ;[1 1 1] Move the Actor based on maths
  (Transformation|SetActorLocation (Math|Vector|MakeVector _x (+ (* (+ (.Y (Math|Vector|BreakVector _location)) (Variables|Default|GetStartingHeight)) (Variables|Default|GetMoveSpeed)) _y) _z) false false))

(fn AssignDATracker
  (params (DATracker :type DA%20Tracker%20Object%20Reference))
  (Variables|Default|SetDA_Tracker DATracker))