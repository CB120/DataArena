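; Level manager that spawns the tracker actors and player pairs, handles level fades and accumulates player points.
; On BeginPlay it creates linked DA and physical trackers from GameInstanceDAGR's IDs and rotation offsets, then assigns them to PlayerPairClass instances two apiece in index order.
; It also fades in and repositions cameras, with CameraActor moved after a delay.
; FadeOut starts the fade and adds level points to the game instance totals.
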(event EventBeginPlay
  (bind _returnvalue (Math|Transform|MakeTransform "0, 0, 0"))
  (Utilities|FlowControl|Sequence
    (:then_0
      ;[1 1 1] Make out list of tracker IDs match that of the game instance (so we know which players own which trackers)
      (bind _asgame_instance_dagr (Utilities|Casting|CastToGameInstanceDAGR (Game|GetGameInstance)))
      (Variables|Default|SettrackerIDs (Variables|/Game/Blueprints/GameInstanceDAGR.GameInstanceDAGR_C|GettrackerIDs _asgame_instance_dagr))
      ;[1 1 1] Create 8 DA trackers, and store references to them
      (for (_array_element _array_index) (Variables|Default|GettrackerIDs)
        (bind _returnvalue_2 (Game|SpawnActorfromClass "/DA_Assets/DeviceCommunication/DA_Tracker.DA_Tracker_C" _returnvalue "Undefined" 0 _array_element 0))
        (bind _returnvalue_3 (Game|SpawnActorfromClass "/Game/Blueprints/Physical_Tracker.Physical_Tracker_C" _returnvalue "Undefined" 0 _array_element _returnvalue_2 (Utilities|Array|Get(acopy) (Variables|/Game/Blueprints/GameInstanceDAGR.GameInstanceDAGR_C|GetrotationOffsets _asgame_instance_dagr) _array_index) (Variables|Default|GettrackersCopyDATrackers) 0))
        (Development|SetHiddeninGame (Variables|/Game/Blueprints/Physical_Tracker.Physical_Tracker_C|GetCone _returnvalue_3) (not (Variables|Default|GettrackersVisible)) false)
        (Utilities|Array|SetArrayElem (Variables|Default|Gettrackers) _array_index _returnvalue_3 true)))
    (:then_1
      ;[1 1 1] Create 4 player pairs (i.e. specified player pair child), and - reading recorded player pair info - set references to respective DA trackers in each player pair object
      (if (Utilities|IsValidClass (Variables|Default|GetplayerPairClass))
        (for (_ _array_index_2) (Variables|Default|GetplayerPairs)
          (bind _returnvalue_4 (Game|SpawnActorfromClass (Variables|Default|GetplayerPairClass) _returnvalue "AlwaysSpawn" 0 0))
          (bind _asplayer_pair (Utilities|Casting|CastToPlayerPair _returnvalue_4))
          (Utilities|Array|SetArrayElem (Variables|Default|GetplayerPairs) _array_index_2 _asplayer_pair true)
          (Default|AssignTrackersandNumber _asplayer_pair (Utilities|Array|Get(acopy) (Variables|Default|Gettrackers) (* _array_index_2 2)) (Utilities|Array|Get(acopy) (Variables|Default|Gettrackers) (+ (* _array_index_2 2) 1)) _array_index_2))
        (else
          (Development|PrintString "No playerPairClass set in PlayerManager!"))))
    (:then_2
      (CallFunction|Fadein))
    (:then_3
      ;[1 1 1] Move the space mouse camera to a default world position on level load
      (if (Variables|Default|GetSetCamLocationOnStart)
        (Utilities|FlowControl|Sequence
          (:then_0
            (bind _returnvalue_5 (Actor|GetActorOfClass "/DA_Assets/Camera/SpaceMouseCamera.SpaceMouseCamera_C"))
            (if (Utilities|IsValid _returnvalue_5)
              (Transformation|SetActorLocation _returnvalue_5 (Variables|Default|GetspaceMouseCameraPosition) false false)))
          (:then_1
            (Utilities|FlowControl|Delay 1.0 :!label _label)
            (bind _returnvalue_6 (Actor|GetActorOfClass "/Script/Engine.CameraActor"))
            (if (Utilities|IsValid _returnvalue_6)
              (Transformation|SetActorLocation _returnvalue_6 (Variables|Default|GetspaceMouseCameraPosition) false false))))
        (else
          (goto _label))))))

(event Collision|EventActorBeginOverlap
  (params (OtherActor :type Actor%20Object%20Reference)))

(event EventTick
  (params (DeltaSeconds :type Float%20%28single-precision%29)))

(fn ConstructionScript)

(fn Fadein
  (bind _returnvalue (UserInterface|CreateWidget "/Game/Blueprints/FadeInOutWidget.FadeInOutWidget_C"))
  (UserInterface|Viewport|AddtoViewport _returnvalue 0)
  (Default|BeginFadeLevelin _returnvalue))

(fn FadeOut
  (bind _returnvalue (UserInterface|CreateWidget "/Game/Blueprints/FadeInOutWidget.FadeInOutWidget_C"))
  (UserInterface|Viewport|AddtoViewport _returnvalue 0)
  (Default|BeginFadeLevelOut _returnvalue)
  (CallFunction|AddPointstoCumulativePointTotal))

(fn AddPointstoCumulativePointTotal
  (bind _asgame_instance_dagr (Utilities|Casting|CastToGameInstanceDAGR (Game|GetGameInstance)))
  (for (_array_element _array_index) (Variables|/Game/Blueprints/GameInstanceDAGR.GameInstanceDAGR_C|GetplayerPoints _asgame_instance_dagr)
    (Utilities|Array|SetArrayElem (Variables|/Game/Blueprints/GameInstanceDAGR.GameInstanceDAGR_C|GetplayerPoints _asgame_instance_dagr) _array_index (+ _array_element (Utilities|Array|Get(acopy) (Variables|Default|GetplayerPoints) _array_index)))))