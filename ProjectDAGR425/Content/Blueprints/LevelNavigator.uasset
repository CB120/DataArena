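; LevelNavigator switches between levels listed in GameInstanceDAGR through Left/Right keys or bound button events.
; Both inputs call LoadAdjacentLevel with a direction, which offsets the current level's index modulo the list length.
; A negative result wraps from the list's end, but any other result opens the first entry rather than the computed neighbour.
; BeginPlay caches a camera owner, but the vertical camera movement logic is unconnected.
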(event Custom|Load%20Level%20to%20Left
  (CallFunction|LoadAdjacentLevel -1))

(event Custom|Load%20Level%20To%20Right
  (CallFunction|LoadAdjacentLevel 1))

(event EventBeginPlay
  (EventDispatchers|BindEventtoLeftButtonPressed (delegate Custom|Load%20Level%20to%20Left))
  (EventDispatchers|BindEventtoRightButtonPressed (delegate Custom|Load%20Level%20To%20Right))
  (Variables|Default|SetCamera (Components|GetOwner (Actor|GetComponentbyClass "/Script/Engine.CameraComponent"))))

(event Collision|EventActorBeginOverlap
  (params (OtherActor :type Actor%20Object%20Reference)))

(event EventTick
  (params (DeltaSeconds :type Float%20%28single-precision%29)))

(event Input|KeyboardEvents|Left
  (params (Key :type Key%20Structure :default "None"))
  (:Pressed
    (CallFunction|LoadAdjacentLevel -1)))

(event Input|KeyboardEvents|Right
  (params (Key :type Key%20Structure :default "None"))
  (:Pressed
    (CallFunction|LoadAdjacentLevel 1)))

(fn ConstructionScript)

(fn LoadAdjacentLevel
  (params (direction :type Integer))
  (bind _asgame_instance_dagr (Utilities|Casting|CastToGameInstanceDAGR (Game|GetGameInstance)))
  (bind _returnvalue (Game|GetCurrentLevelName true))
  (if (< (Math|Integer|%(Integer) (+ (Utilities|Array|FindItem (Variables|/Game/Blueprints/GameInstanceDAGR.GameInstanceDAGR_C|GetlevelNames _asgame_instance_dagr) _returnvalue) direction) (Utilities|Array|Length (Variables|/Game/Blueprints/GameInstanceDAGR.GameInstanceDAGR_C|GetlevelNames _asgame_instance_dagr))) 0)
    (Game|OpenLevel(byName) (Utilities|String|StringToName (Utilities|Array|Get(acopy) (Variables|/Game/Blueprints/GameInstanceDAGR.GameInstanceDAGR_C|GetlevelNames _asgame_instance_dagr) (+ (Utilities|Array|Length (Variables|/Game/Blueprints/GameInstanceDAGR.GameInstanceDAGR_C|GetlevelNames _asgame_instance_dagr)) (Math|Integer|%(Integer) (+ (Utilities|Array|FindItem (Variables|/Game/Blueprints/GameInstanceDAGR.GameInstanceDAGR_C|GetlevelNames _asgame_instance_dagr) _returnvalue) direction) (Utilities|Array|Length (Variables|/Game/Blueprints/GameInstanceDAGR.GameInstanceDAGR_C|GetlevelNames _asgame_instance_dagr)))))))
    (else
      (Game|OpenLevel(byName) (Utilities|String|StringToName (Utilities|Array|Get(acopy) (Variables|/Game/Blueprints/GameInstanceDAGR.GameInstanceDAGR_C|GetlevelNames _asgame_instance_dagr)))))))