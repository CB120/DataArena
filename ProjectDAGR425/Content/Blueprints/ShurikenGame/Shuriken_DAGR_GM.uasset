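; Game mode for a timed shuriken match that ends the round and announces the highest-scoring player.
; It shows a timer widget, counts GameLength down every Tick and feeds the remaining time to the widget.
; At zero it scans PlayerManager's points once, passes the winner's index and color to its delayed fade-out, and removes the timer.
; Ties with the running high score only print a stalemate message; the earlier player remains winner.
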(event EventBeginPlay
  (|CallParentFunction)
  (bind _returnvalue (UserInterface|CreateWidget "/Game/BowArrow/MatchTimeWidget.MatchTimeWidget_C"))
  (UserInterface|Viewport|AddtoViewport _returnvalue 0)
  (bind _output_get (Variables|Default|SettimerWidget _returnvalue))
  (Variables|/Game/BowArrow/MatchTimeWidget.MatchTimeWidget_C|SetgameTime _output_get (Variables|Default|GetGameLength)))

(event EventTick
  (params (DeltaSeconds :type Float%20%28single-precision%29))
  (|CallParentFunction DeltaSeconds)
  (bind _output_get (Variables|Default|SetGameLength (- (Variables|Default|GetGameLength) DeltaSeconds)))
  (if (<= (Variables|Default|GetGameLength) 0.0)
    (if (not (Variables|Default|GetgameEnded))
      (Variables|Default|SetgameEnded true)
      (bind _returnvalue (Actor|GetActorOfClass "/Game/Blueprints/PlayerManager.PlayerManager_C"))
      (for (_array_element _array_index) (Variables|/Game/Blueprints/PlayerManager.PlayerManager_C|GetplayerPoints _returnvalue)
        (if (> _array_element (Variables|Default|GetHighestPoints))
          (Variables|Default|SetHighestPoints _array_element)
          (Variables|Default|SetCurrentWinner _array_index)
          (elif (== _array_element (Variables|Default|GetHighestPoints))
            (Development|PrintString "Stale mate!"))))
      (bind _color (Default|GetPlayerColor (Utilities|Array|Get(acopy) (Variables|/Game/Blueprints/PlayerManager.PlayerManager_C|GetplayerPairs _returnvalue) (Variables|Default|GetCurrentWinner))))
      (Default|DelayedFadeOut _returnvalue (Variables|Default|GetCurrentWinner) (Math|Conversions|ToColor(LinearColor) _color) 0.0)
      (Widget|RemovefromParent (Variables|Default|GettimerWidget)))
    (else
      (Variables|/Game/BowArrow/MatchTimeWidget.MatchTimeWidget_C|SetgameTime (Variables|Default|GettimerWidget) (Variables|Default|GetGameLength)))))

(fn ConstructionScript
  (|CallParentFunction))