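; Player actor for the shuriken game that detects a two-handed throwing gesture from motion trackers, currently only partly wired.
; Tracker activation sets the reload flag, and Tick checks hand proximity, then alignment via dot products of tracker forwards and the between-hands vector.
; An uncalled reticle helper places a widget at a line-trace hit, facing the SpaceMouse camera.
; FireShuriken is empty, with its spawn-and-impulse logic disconnected, so nothing is thrown.
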(event Custom|RightHand%20Reload
  (Variables|Default|SetisReloaded true))

(event EventBeginPlay
  (bind _asda_tracker (Utilities|Casting|CastToDA_Tracker (Variables|Default|GetTrackerR)))
  (EventDispatchers|BindEventtoTrackerActivated _asda_tracker (delegate Custom|RightHand%20Reload)))

(event EventTick
  (params (DeltaSeconds :type Float%20%28single-precision%29))
  (Utilities|FlowControl|Sequence
    (:then_0
      (bind _readytothrow (CallFunction|CheckThrowingStance))
      (if _readytothrow
        (if (Variables|Default|GetisReloaded)
          ;[1 1 1] This needs to be modified to work with shooting out
          (bind _iscorrectlyangled (CallFunction|IsCorrectlyAngled))
          (if _iscorrectlyangled
            _)
          (else
            (Development|PrintString "Reload!!")))))
    (:then_1
      (if (Variables|Default|GetisReloaded)
        _))))

(fn ConstructionScript
  (|CallParentFunction))

(fn GetPointDirection
  ;[1 1 1] Logic courtesy of Eddie
  (bind _vectorpointing (CallFunction|GetVectorBetweenTrackers "NewEnumerator0" true))
  (return _vectorpointing))

(fn IsCorrectlyAngled
  ;[1 1 1] Logic courtesy of Eddie
  (Utilities|FlowControl|Sequence
    (:then_0
      ;[1 1 1] Are both hands pointing in similar directions?
      (bind _dotproduct (CallFunction|GetDotProductOfTrackerForwardVectors)))
    (:then_1
      ;[1 1 1] Are both hands pointing in a similar enough direction to the vector formed between their hands?
      (bind _forwardvector (CallFunction|GetTrackerForwardVector "NewEnumerator0"))
      (bind _forwardvector_2 (CallFunction|GetTrackerForwardVector "NewEnumerator1"))
      (bind _pointdirection (CallFunction|GetPointDirection))
      (return (and (>= _dotproduct 0.8) (>= (Math|Vector|DotProduct _pointdirection (Math|Vector|Lerp(Vector) _forwardvector _forwardvector_2 0.5)) 0.65))))))

(fn CheckThrowingStance
  ;[1 1 1] Record if both hands are close together
  (bind _distance (CallFunction|GetDistanceBetweenTrackers))
  (bind _output_get (Variables|Default|SetReadyToThrow (<= _distance 0.0)))
  (return _output_get))

(fn UpdateReticle
  (params (IsVisible :type Boolean) (PlayerPosition :type Vector) (PointDirection :type Vector))
  (bind _widget (Variables|Default|GetWidget))
  (Utilities|FlowControl|Sequence
    (:then_0
      (Rendering|SetVisibility (Variables|Default|GetWidget) IsVisible false))
    (:then_1
      (if true
        ;[1 1 1] Draw ray trace
        (bind _outhit (Collision|LineTraceByChannel (+ PlayerPosition (* PointDirection 5e+01)) (+ PlayerPosition (* PointDirection 1e+03)) "TraceTypeQuery1" false 0 "None"))
        (Transformation|SetWorldLocation (Variables|Default|GetWidget) (.Location (Collision|BreakHitResult _outhit)) false false)
        ;[1 1 1] Why are we fetching this every tick...?
        (bind _returnvalue (Actor|GetActorOfClass "/DA_Assets/Camera/SpaceMouseCamera.SpaceMouseCamera_C"))
        (Utilities|IsValid _returnvalue
          (:Is%20Valid
            ;[1 1 1] Billboard reticle towards where we think the camera is
            (Transformation|SetWorldRotation _widget (Math|Rotator|FindLookatRotation (.Location (Collision|BreakHitResult _outhit)) (Transformation|GetActorLocation _returnvalue)) false false))
          (:Is%20Not%20Valid
            (Transformation|SetWorldRotation _widget (Math|Rotator|FindLookatRotation (.Location (Collision|BreakHitResult _outhit)) (Math|Vector|MakeVector 0.0 0.0 1.2e+02)) false false)))))))

(fn FireShuriken)