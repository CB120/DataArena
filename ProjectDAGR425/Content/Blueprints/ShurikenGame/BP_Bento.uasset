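; BP_Bento is a bento box penalty object in the shuriken game that costs a player one point when sliced.
; Its construction script copies the static mesh into a procedural mesh with collision.
; Sliced takes a PlayerID, decrements that player's entry in the PlayerManager's PlayerPoints and prints the new total.
; The actor destroys itself three seconds after BeginPlay if the procedural mesh is valid.
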(event EventBeginPlay
  (Utilities|FlowControl|Delay 3.0)
  (Utilities|IsValid (Variables|Default|GetProceduralMesh)
    (:Is%20Valid
      (Actor|DestroyActor))))

(fn ConstructionScript
  (Class|KismetProceduralMeshLibrary|CopyProceduralMeshfromStaticMeshComponent (Variables|Default|GetStaticMesh) 0 (Variables|Default|GetProceduralMesh) true))

(fn Sliced
  (params (playerID :type Integer))
  (bind _returnvalue (Actor|GetActorOfClass "/Game/Blueprints/PlayerManager.PlayerManager_C"))
  (Utilities|Array|SetArrayElem (Variables|/Game/Blueprints/PlayerManager.PlayerManager_C|GetplayerPoints _returnvalue) playerID (- (Utilities|Array|Get(acopy) (Variables|/Game/Blueprints/PlayerManager.PlayerManager_C|GetplayerPoints _returnvalue) playerID) 1))
  (Development|PrintString (Utilities|String|Append "Player " (Utilities|String|ToString(Integer) playerID) " has sliced a bento box! minus 1 point. " " total = " (Utilities|String|ToString(Integer) (Utilities|Array|Get(acopy) (Variables|/Game/Blueprints/PlayerManager.PlayerManager_C|GetplayerPoints _returnvalue) playerID))) true true "(R=0.000000,G=0.660000,B=1.000000,A=1.000000)" 3.0))