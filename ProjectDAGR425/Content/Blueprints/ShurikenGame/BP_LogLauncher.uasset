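; BP_LogLauncher is a shuriken game launcher that repeatedly throws objects upward from its spawn point.
; From BeginPlay it spawns a scaled-up BP_Log, applies an upward impulse to its procedural mesh and emits gun smoke, looping after a random delay of a few seconds.
; An alternate branch floats a gravity-free BP_Bento, but the random weight of 1.0 always selects the log.
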(event EventBeginPlay
  (bind _spawnpoint (Variables|Default|GetSpawnPoint))
  (bind _returnvalue (Transformation|GetWorldTransform _spawnpoint))
  (if (Math|Random|RandomBoolwithWeight 1.0) :!label _label
    (bind _returnvalue_2 (Game|SpawnActorfromClass "/Game/Blueprints/ShurikenGame/BP_Log.BP_Log_C" (Math|Transform|MakeTransform (+ (.location _returnvalue) "0, 0,100.000000") "0, 0, 0" "4.000000,4.000000,4.000000") "Undefined" 0 0))
    (Physics|AddImpulseatLocation (Variables|/Game/Blueprints/ShurikenGame/BP_Log.BP_Log_C|GetProceduralMesh _returnvalue_2) (Math|Vector|MakeVector 0.0 0.0 4e+03) (Transformation|GetWorldLocation (Variables|/Game/Blueprints/ShurikenGame/BP_Log.BP_Log_C|GetProceduralMesh _returnvalue_2)) "")
    (Effects|SpawnEmitteratLocation "/Game/Assets/Christian-Assets/P_GunSmoke.P_GunSmoke" (.location _returnvalue) "0, 0, 0" "2.000000,2.000000,2.000000")
    (else
      (bind _returnvalue_3 (Game|SpawnActorfromClass "/Game/Blueprints/ShurikenGame/BP_Bento.BP_Bento_C" (Math|Transform|MakeTransform (.location _returnvalue) "0, 0, 0" "0.500000,0.500000,0.500000") "Undefined" 0 0))
      (Physics|AddImpulseatLocation (Variables|/Game/Blueprints/ShurikenGame/BP_Bento.BP_Bento_C|GetProceduralMesh _returnvalue_3) "0, 0,20.000000" (Transformation|GetWorldLocation (Variables|/Game/Blueprints/ShurikenGame/BP_Bento.BP_Bento_C|GetProceduralMesh _returnvalue_3)) "None")
      (Physics|SetEnableGravity (Variables|/Game/Blueprints/ShurikenGame/BP_Bento.BP_Bento_C|GetProceduralMesh _returnvalue_3) false)
      (Utilities|FlowControl|Delay 1.0)
      (Physics|SetEnableGravity (Variables|/Game/Blueprints/ShurikenGame/BP_Bento.BP_Bento_C|GetProceduralMesh _returnvalue_3) false)))
  (Utilities|FlowControl|Delay (Math|Random|RandomFloatinRange 4.0 5.5))
  (goto _label))

(fn ConstructionScript)