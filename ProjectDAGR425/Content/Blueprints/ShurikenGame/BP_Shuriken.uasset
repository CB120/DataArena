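; BP_Shuriken is a thrown shuriken projectile that slices procedural meshes it overlaps.
; On BeginPlay it launches with a physics impulse and destroys itself after a few seconds, while Tick spins it.
; Overlap cuts the mesh along the Plane component with a capped face, then pushes the new half away and removes it after a delay.
; A DoOnce, reset on end overlap, prevents repeated cuts during an overlap.
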(event OnComponentBeginOverlap(Shuriken)
  (params (OverlappedComponent :type Primitive%20Component%20Object%20Reference) (OtherActor :type Actor%20Object%20Reference) (OtherComp :type Primitive%20Component%20Object%20Reference) (OtherBodyIndex :type Integer) (bFromSweep :type Boolean) (SweepResult :type Hit%20Result%20Structure%20%28by%20ref%29))
  (bind _plane (Variables|Default|GetPlane))
  (bind _returnvalue (Transformation|GetWorldLocation _plane))
  (Utilities|FlowControl|DoOnce false
    (:Completed
      (bind _asprocedural_mesh_component (Utilities|Casting|CastToProceduralMeshComponent OtherComp))
      (bind _outotherhalfprocmesh (Class|KismetProceduralMeshLibrary|SliceProceduralMesh _asprocedural_mesh_component _returnvalue (Math|Vector|GetUpVector _plane) true "CreateNewSectionForCap" "/Game/Assets/Christian-Assets/Material__2.Material__2"))
      (Physics|SetSimulatePhysics _outotherhalfprocmesh true)
      (Physics|AddRadialImpulse _outotherhalfprocmesh _returnvalue 2.5e+02 6.5e+02 "RIF_Constant" false)
      (Development|PrintString "Sliced!")
      (Utilities|FlowControl|Delay 1.5)
      (Utilities|IsValid _outotherhalfprocmesh
        (:Is%20Valid
          (Components|DestroyComponent _outotherhalfprocmesh))))))

(event OnComponentEndOverlap(Shuriken)
  (params (OverlappedComponent :type Primitive%20Component%20Object%20Reference) (OtherActor :type Actor%20Object%20Reference) (OtherComp :type Primitive%20Component%20Object%20Reference) (OtherBodyIndex :type Integer))
  (bind _plane (Variables|Default|GetPlane))
  (bind _returnvalue (Transformation|GetWorldLocation _plane))
  (Utilities|FlowControl|DoOnce false) ; enters at Reset
)

(event EventBeginPlay
  (bind _shuriken (Variables|Default|GetShuriken))
  (Physics|SetSimulatePhysics _shuriken true)
  (Physics|AddImpulse _shuriken (* (Class|KismetMathLibrary|VectorForward) 35000) "None" false)
  (Utilities|FlowControl|Delay 3.0)
  (Actor|DestroyActor))

(event Collision|EventActorBeginOverlap
  (params (OtherActor :type Actor%20Object%20Reference)))

(event EventTick
  (params (DeltaSeconds :type Float%20%28single-precision%29))
  (Transformation|AddLocalRotation (Variables|Default|GetShuriken) (Math|Rotator|MakeRotator 0.0 0.0 (+ 0.0 4.0)) false false))

(fn ConstructionScript)