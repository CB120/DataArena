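; Manages an nDisplay shadow-matching game, spawning a ring of frames and a player/target pair of random shapes per player.
; The master node spawns the initial pairs and broadcasts cluster events from which other nodes build proxy shadows.
; Each tick, player trackers drive shadow yaw and distance from the center.
; Pairs matching in rotation and apparent size (distance versus scale ratio) print a score and respawn locally, without a cluster event.
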(event EventBeginPlay
  (bind _outapi (Class|DisplayClusterBlueprintLib|GetAPI))
  (bind _number_of_players (Variables|Default|GetNumber%20of%20Players))
  (Class|DisplayClusterBlueprintAPI|AddClusterEventListener _outapi self)
  (CallFunction|SpawnAllFrames _number_of_players)
  (bind _returnvalue (Class|DisplayClusterBlueprintAPI|IsMaster _outapi))
  (if _returnvalue
    (CallFunction|SpawnPlayerShadows _number_of_players)
    (CallFunction|SpawnTargetShadows _number_of_players)))

(event Collision|EventActorBeginOverlap
  (params (OtherActor :type Actor%20Object%20Reference)))

(event EventTick
  (params (DeltaSeconds :type Float%20%28single-precision%29))
  (CallFunction|UpdatePlayerShadows)
  (CallFunction|CheckPlayerShadows))

(event EventOnClusterEvent
  (params (Event :type Display%20Cluster%20Cluster%20Event%20Structure%20%28by%20ref%29))
  (bind _outapi (Class|DisplayClusterBlueprintLib|GetAPI))
  (switch string (.name Event)
    (:Spawn%20Player%20Shadow
      (bind _returnvalue (Class|DisplayClusterBlueprintAPI|IsMaster _outapi))
      (if (not _returnvalue)
        (CallFunction|SpawnProxyShadow (.parameters Event) false)))
    (:Spawn%20Target%20Shadow
      (bind _returnvalue_2 (Class|DisplayClusterBlueprintAPI|IsMaster _outapi))
      (if (not _returnvalue_2)
        (CallFunction|SpawnProxyShadow (.parameters Event) true)))))

(fn ConstructionScript)

(fn SpawnSingleShadow
  (params (Shadow%20Class :type Shadow%20Scale%20Struct%20Structure) (Location :type Vector) (Angle :type Float%20%28single-precision%29) (Pitch :type Float%20%28single-precision%29) (Roll :type Float%20%28single-precision%29) (Yaw :type Float%20%28single-precision%29) (Has%20Authority :type Boolean))
  (bind _returnvalue (Math|Random|RandomFloatinRange 0.0 3.6e+02))
  (bind _returnvalue_2 (Math|Float|SelectFloat _returnvalue Yaw Has%20Authority))
  (bind _returnvalue_3 (Game|SpawnActorfromClass (.shadowclass Shadow%20Class) (Math|Transform|MakeTransform Location (Math|Rotator|MakeRotator 0.0 0.0 Angle) (Math|Vector|Lerp(Vector) (* "1.000000,1.000000,1.000000" (.minimumscale Shadow%20Class)) (* "1.000000,1.000000,1.000000" (.maximumscale Shadow%20Class)) 0.5)) "Undefined" 0 0))
  (bind _model (CallFunction|GetModel _returnvalue_3))
  (Transformation|SetRelativeRotation _model (Math|Rotator|MakeRotator Roll Pitch _returnvalue_2) false false)
  (return _returnvalue_3 Pitch Roll _returnvalue_2))

(fn GetRandomShadowClass
  (bind _shadow_classes (Variables|Default|GetShadow%20Classes))
  (bind _returnvalue (Utilities|Array|Length _shadow_classes))
  (bind _returnvalue_2 (- _returnvalue 1))
  (bind _returnvalue_3 (Math|Random|RandomIntegerinRange 0 _returnvalue_2))
  (return (Utilities|Array|Get(acopy) _shadow_classes _returnvalue_3) _returnvalue_3))

(fn GetRandomSpawnLocation
  (params (Angle :type Float%20%28single-precision%29))
  (bind _minimum_spawn_distance (Variables|Default|GetMinimum%20Spawn%20Distance))
  (bind _maximum_spawn_distance (Variables|Default|GetMaximum%20Spawn%20Distance))
  (bind _returnvalue (Math|Random|RandomFloatinRange _minimum_spawn_distance _maximum_spawn_distance))
  (return (Math|Vector|MakeVector (* (Math|Trig|Cos(Degrees) Angle) _returnvalue) (* _returnvalue (Math|Trig|Sin(Degrees) Angle)) (Math|Random|RandomFloatinRange 1.4e+02 1.6e+02))))

(fn SpawnAllFrames
  (params (Number%20of%20Players :type Integer))
  (bind _output_get (LocalVariables|SetPlayers Number%20of%20Players))
  (bind _output_get_2 (LocalVariables|SetFrames (* _output_get 2)))
  (for _index (range 0 (- _output_get_2 1))
    (LocalVariables|SetIndex _index)
    (bind _output_get_3 (LocalVariables|SetAngle (* (/ 3.6e+02 (Math|Conversions|ToFloat(Integer) (LocalVariables|GetFrames))) (Math|Conversions|ToFloat(Integer) (LocalVariables|GetIndex))))) ; Increments the angle evenly
    (bind _output_get_4 (LocalVariables|SetIs%20Even (== (Math|Integer|%(Integer) (LocalVariables|GetIndex) 2) 0)))
    (CallFunction|SpawnFrame _output_get_3 _output_get_4)))

(fn SpawnFrame
  (params (Angle :type Float%20%28single-precision%29) (Is%20Even :type Boolean))
  (bind _location (CallFunction|GetSpawnLocation Angle (Math|Float|SelectFloat 2e+02 2.6e+02 Is%20Even)))
  (Game|SpawnActorfromClass "/Game/Blueprints/ShadowShapes/ShadowFrame.ShadowFrame_C" (Math|Transform|MakeTransform _location (Math|Rotator|MakeRotator (Math|Float|SelectFloat 0.0 45.0 Is%20Even) 0.0 Angle) "1,1,1") "Undefined" 0 0))

(fn GetSpawnLocation
  (params (Angle :type Float%20%28single-precision%29) (Distance :type Float%20%28single-precision%29))
  (return (Math|Vector|MakeVector (* (Math|Trig|Cos(Degrees) Angle) Distance) (* Distance (Math|Trig|Sin(Degrees) Angle)) 1.5e+02)))

(fn SpawnPlayerShadows
  (params (Number%20of%20Players :type Integer))
  (bind _returnvalue (Math|Random|RandomRotator true))
  (bind _minimum_spawn_distance (Variables|Default|GetMinimum%20Spawn%20Distance))
  (bind _maximum_spawn_distance (Variables|Default|GetMaximum%20Spawn%20Distance))
  (bind _returnvalue_2 (Math|Random|RandomFloatinRange _minimum_spawn_distance _maximum_spawn_distance))
  (bind _output_get (LocalVariables|SetPlayers Number%20of%20Players))
  (for _index (range 0 (- _output_get 1))
    (LocalVariables|SetIndex _index)
    (bind _output_get_2 (LocalVariables|SetAngle (* (/ 3.6e+02 (Math|Conversions|ToFloat(Integer) (LocalVariables|GetPlayers))) (Math|Conversions|ToFloat(Integer) (LocalVariables|GetIndex)))))
    (bind _location (CallFunction|GetSpawnLocation _output_get_2 _returnvalue_2))
    (bind (_shadow_class _index_2) (CallFunction|GetRandomShadowClass))
    (bind (_shadow _pitch_output _roll_output _yaw_output) (CallFunction|SpawnSingleShadow _shadow_class _location (LocalVariables|GetAngle) (.pitch _returnvalue) (.roll _returnvalue) 0.0 true))
    (bind _direction (CallFunction|GetDirectionfromAngle (LocalVariables|GetAngle)))
    (bind _returnvalue_3 (Utilities|Array|Add (Variables|Default|GetShadow%20Pairs) (Utilities|Struct|MakeShadowPair _shadow 0 _shadow_class (LocalVariables|GetAngle) 0.0 _direction _pitch_output _roll_output)))
    (Class|DisplayClusterBlueprintAPI|EmitClusterEvent (Class|DisplayClusterBlueprintLib|GetAPI) (Utilities|Struct|MakeDisplayClusterClusterEvent "Spawn Player Shadow" "" "" (Utilities|Map|MakeMap "Player" (Utilities|String|ToString(Integer) (LocalVariables|GetIndex)) "Shadow" (Utilities|String|ToString(Integer) _index_2) "Distance" (Utilities|String|ToString(Float) _returnvalue_2) "Pitch" (Utilities|String|ToString(Float) (.pitch _returnvalue)) "Roll" (Utilities|String|ToString(Float) (.roll _returnvalue)) "Yaw" (Utilities|String|ToString(Float) _yaw_output) "Index" (Utilities|String|ToString(Integer) _returnvalue_3))) false)))

(fn SpawnTargetShadows
  (params (Number%20Of%20Players :type Integer))
  (bind _minimum_spawn_distance (Variables|Default|GetMinimum%20Spawn%20Distance))
  (bind _maximum_spawn_distance (Variables|Default|GetMaximum%20Spawn%20Distance))
  (bind _returnvalue (Math|Random|RandomFloatinRange _minimum_spawn_distance _maximum_spawn_distance))
  (bind _output_get (LocalVariables|SetPlayers Number%20Of%20Players))
  (for _index (range 0 (- _output_get 1))
    (LocalVariables|SetIndex _index)
    (LocalVariables|SetAngle (+ (* (/ 3.6e+02 (Math|Conversions|ToFloat(Integer) (LocalVariables|GetPlayers))) (Math|Conversions|ToFloat(Integer) (LocalVariables|GetIndex))) (/ 1.8e+02 (Math|Conversions|ToFloat(Integer) (LocalVariables|GetPlayers)))))
    (bind _pair_index (CallFunction|GetPairIndexfromTargetIndex (LocalVariables|GetIndex)))
    (bind _output_get_2 (LocalVariables|SetPair%20Index _pair_index))
    (bind _location (CallFunction|GetSpawnLocation (LocalVariables|GetAngle) _returnvalue))
    (bind (_shadow _pitch_output _roll_output _yaw_output) (CallFunction|SpawnSingleShadow (.sourceclass (Utilities|Array|Get(acopy) (Variables|Default|GetShadow%20Pairs) _output_get_2)) _location (LocalVariables|GetAngle) (.pitch (Utilities|Array|Get(acopy) (Variables|Default|GetShadow%20Pairs) (LocalVariables|GetPair%20Index))) (.roll (Utilities|Array|Get(acopy) (Variables|Default|GetShadow%20Pairs) (LocalVariables|GetPair%20Index))) 0.0 true))
    (Utilities|Array|SetArrayElem (Variables|Default|GetShadow%20Pairs) (LocalVariables|GetPair%20Index) (Utilities|Struct|MakeShadowPair (.playershadow (Utilities|Array|Get(acopy) (Variables|Default|GetShadow%20Pairs) (LocalVariables|GetPair%20Index))) _shadow (.sourceclass (Utilities|Array|Get(acopy) (Variables|Default|GetShadow%20Pairs) (LocalVariables|GetPair%20Index))) (.playerangle (Utilities|Array|Get(acopy) (Variables|Default|GetShadow%20Pairs) (LocalVariables|GetPair%20Index))) (LocalVariables|GetAngle) (.playerdirection (Utilities|Array|Get(acopy) (Variables|Default|GetShadow%20Pairs) (LocalVariables|GetPair%20Index))) (.pitch (Utilities|Array|Get(acopy) (Variables|Default|GetShadow%20Pairs) (LocalVariables|GetPair%20Index))) (.roll (Utilities|Array|Get(acopy) (Variables|Default|GetShadow%20Pairs) (LocalVariables|GetPair%20Index)))))
    (Class|DisplayClusterBlueprintAPI|EmitClusterEvent (Class|DisplayClusterBlueprintLib|GetAPI) (Utilities|Struct|MakeDisplayClusterClusterEvent "Spawn Target Shadow" "" "" (Utilities|Map|MakeMap "Player" (Utilities|String|ToString(Integer) (LocalVariables|GetIndex)) "Shadow" (Utilities|String|ToString(Integer) (Utilities|Array|FindItem (Variables|Default|GetShadow%20Classes) (.sourceclass (Utilities|Array|Get(acopy) (Variables|Default|GetShadow%20Pairs) (LocalVariables|GetPair%20Index))))) "Distance" (Utilities|String|ToString(Float) _returnvalue) "Pitch" (Utilities|String|ToString(Float) _pitch_output) "Roll" (Utilities|String|ToString(Float) _roll_output) "Yaw" (Utilities|String|ToString(Float) _yaw_output) "Index" (Utilities|String|ToString(Integer) (LocalVariables|GetPair%20Index)))) false)))

(fn GetPairIndexfromTargetIndex
  (params (Target%20Index :type Integer))
  (bind _output_get (LocalVariables|SetOutput (- Target%20Index 1)))
  (if (< _output_get 0)
    (LocalVariables|SetOutput (- (Variables|Default|GetNumber%20of%20Players) 1)))
  (return (LocalVariables|GetOutput)))

(fn CheckPlayerShadows
  (for (_array_element _array_index) (Variables|Default|GetShadow%20Pairs)
    (LocalVariables|SetIndex _array_index)
    (bind _passed_rotation_check (CallFunction|CompareRotations (.playershadow _array_element) (.targetshadow _array_element)))
    (if _passed_rotation_check
      (bind _passed_shadow_size_check (CallFunction|CompareShadowSize (.playershadow _array_element) (.targetshadow _array_element)))
      (if _passed_shadow_size_check
        (Development|PrintString (Utilities|String|Append "Player " (Utilities|String|ToString(Integer) (LocalVariables|GetIndex)) "Scored!"))
        (Actor|DestroyActor (.playershadow _array_element))
        (Actor|DestroyActor (.targetshadow _array_element))
        (bind _location (CallFunction|GetSpawnLocation (.playerangle (Utilities|Array|Get(acopy) (Variables|Default|GetShadow%20Pairs) (LocalVariables|GetIndex))) (Math|Random|RandomFloatinRange (Variables|Default|GetMinimum%20Spawn%20Distance) (Variables|Default|GetMaximum%20Spawn%20Distance))))
        (bind _shadow_class (CallFunction|GetRandomShadowClass))
        (bind _shadow (CallFunction|SpawnSingleShadow _shadow_class _location (.playerangle (Utilities|Array|Get(acopy) (Variables|Default|GetShadow%20Pairs) (LocalVariables|GetIndex))) 0.0 0.0 0.0 false))
        (bind _location_2 (CallFunction|GetSpawnLocation (.targetangle (Utilities|Array|Get(acopy) (Variables|Default|GetShadow%20Pairs) (LocalVariables|GetIndex))) (Math|Random|RandomFloatinRange (Variables|Default|GetMinimum%20Spawn%20Distance) (Variables|Default|GetMaximum%20Spawn%20Distance))))
        (bind _shadow_2 (CallFunction|SpawnSingleShadow _shadow_class _location_2 (.targetangle (Utilities|Array|Get(acopy) (Variables|Default|GetShadow%20Pairs) (LocalVariables|GetIndex))) 0.0 0.0 0.0 false))
        (Utilities|Array|SetArrayElem (Variables|Default|GetShadow%20Pairs) (LocalVariables|GetIndex) (Utilities|Struct|MakeShadowPair _shadow _shadow_2 _shadow_class (.playerangle (Utilities|Array|Get(acopy) (Variables|Default|GetShadow%20Pairs) (LocalVariables|GetIndex))) (.targetangle (Utilities|Array|Get(acopy) (Variables|Default|GetShadow%20Pairs) (LocalVariables|GetIndex))) "NewEnumerator0" 0.0 0.0))))))

(fn CompareRotations
  (params (Actor%20A :type Actor%20Object%20Reference) (Actor%20B :type Actor%20Object%20Reference))
  (bind _model (CallFunction|GetModel Actor%20A))
  (bind _model_2 (CallFunction|GetModel Actor%20B))
  (return (>= (+ (/ (Math|Vector|DotProduct (Math|Rotator|GetRotationXVector (Variables|/Script/Engine.SceneComponent|GetRelativeRotation _model)) (Math|Rotator|GetRotationXVector (Variables|/Script/Engine.SceneComponent|GetRelativeRotation _model_2))) (+ (Math|Vector|VectorLength (Math|Rotator|GetRotationXVector (Variables|/Script/Engine.SceneComponent|GetRelativeRotation _model))) (Math|Vector|VectorLength (Math|Rotator|GetRotationXVector (Variables|/Script/Engine.SceneComponent|GetRelativeRotation _model_2))))) 0.5) (Variables|Default|GetRotation%20Similarity%20Threshold))))

(fn GetModel
  (params (Shadow :type Actor%20Object%20Reference))
  (bind _output_get (LocalVariables|SetInput Shadow))
  (bind _asshadow_beer_paddle (Utilities|Casting|CastToShadowBeerPaddle _output_get)
    (:then
      (return (Variables|/Game/Blueprints/ShadowShapes/ShadowBeerPaddle.ShadowBeerPaddle_C|GetModel _asshadow_beer_paddle)))
    (:CastFailed
      (bind _asshadow_chair (Utilities|Casting|CastToShadowChair (LocalVariables|GetInput))
        (:then
          (return (Variables|/Game/Blueprints/ShadowShapes/ShadowChair.ShadowChair_C|GetModel _asshadow_chair)))
        (:CastFailed
          (bind _asshadow_coliseum (Utilities|Casting|CastToShadowColiseum (LocalVariables|GetInput))
            (:then
              (return (Variables|/Game/Blueprints/ShadowShapes/ShadowColiseum.ShadowColiseum_C|GetModel _asshadow_coliseum)))
            (:CastFailed
              (bind _asshadow_elephant (Utilities|Casting|CastToShadowElephant (LocalVariables|GetInput))
                (:then
                  (return (Variables|/Game/Blueprints/ShadowShapes/ShadowElephant.ShadowElephant_C|GetModel _asshadow_elephant)))
                (:CastFailed
                  (bind _asshadow_graduation_cap (Utilities|Casting|CastToShadowGraduationCap (LocalVariables|GetInput))
                    (:then
                      (return (Variables|/Game/Blueprints/ShadowShapes/ShadowGraduationCap.ShadowGraduationCap_C|GetModel _asshadow_graduation_cap)))
                    (:CastFailed
                      (bind _asshadow_guitar (Utilities|Casting|CastToShadowGuitar (LocalVariables|GetInput))
                        (:then
                          (return (Variables|/Game/Blueprints/ShadowShapes/ShadowGuitar.ShadowGuitar_C|GetModel _asshadow_guitar)))
                        (:CastFailed
                          (bind _asshadow_harp (Utilities|Casting|CastToShadowHarp (LocalVariables|GetInput))
                            (:then
                              (return (Variables|/Game/Blueprints/ShadowShapes/ShadowHarp.ShadowHarp_C|GetModel _asshadow_harp)))
                            (:CastFailed
                              (bind _asshadow_helicopter (Utilities|Casting|CastToShadowHelicopter (LocalVariables|GetInput))
                                (:then
                                  (return (Variables|/Game/Blueprints/ShadowShapes/ShadowHelicopter.ShadowHelicopter_C|GetModel _asshadow_helicopter)))
                                (:CastFailed
                                  (bind _asshadow_jet (Utilities|Casting|CastToShadowJet (LocalVariables|GetInput))
                                    (:then
                                      (return (Variables|/Game/Blueprints/ShadowShapes/ShadowJet.ShadowJet_C|GetModel _asshadow_jet)))
                                    (:CastFailed
                                      (bind _asshadow_ostrich (Utilities|Casting|CastToShadowOstrich (LocalVariables|GetInput))
                                        (:then
                                          (return (Variables|/Game/Blueprints/ShadowShapes/ShadowOstrich.ShadowOstrich_C|GetModel _asshadow_ostrich)))
                                        (:CastFailed
                                          (bind _asshadow_scooter (Utilities|Casting|CastToShadowScooter (LocalVariables|GetInput))
                                            (:then
                                              (return (Variables|/Game/Blueprints/ShadowShapes/ShadowScooter.ShadowScooter_C|GetModel _asshadow_scooter)))
                                            (:CastFailed
                                              (bind _asshadow_slide (Utilities|Casting|CastToShadowSlide (LocalVariables|GetInput))
                                                (:then
                                                  (return (Variables|/Game/Blueprints/ShadowShapes/ShadowSlide.ShadowSlide_C|GetModel _asshadow_slide)))
                                                (:CastFailed
                                                  (bind _asshadow_sunglasses (Utilities|Casting|CastToShadowSunglasses (LocalVariables|GetInput))
                                                    (:then
                                                      (return (Variables|/Game/Blueprints/ShadowShapes/ShadowSunglasses.ShadowSunglasses_C|GetModel _asshadow_sunglasses)))
                                                    (:CastFailed
                                                      (bind _asshadow_tennis_racket (Utilities|Casting|CastToShadowTennisRacket (LocalVariables|GetInput))
                                                        (:then
                                                          (return (Variables|/Game/Blueprints/ShadowShapes/ShadowTennisRacket.ShadowTennisRacket_C|GetModel _asshadow_tennis_racket)))
                                                        (:CastFailed
                                                          (bind _asshadow_tree (Utilities|Casting|CastToShadowTree (LocalVariables|GetInput))
                                                            (:then
                                                              (return (Variables|/Game/Blueprints/ShadowShapes/ShadowTree.ShadowTree_C|GetModel _asshadow_tree)))
                                                            (:CastFailed
                                                              (bind _asshadow_tricycle (Utilities|Casting|CastToShadowTricycle (LocalVariables|GetInput))
                                                                (:then
                                                                  (return (Variables|/Game/Blueprints/ShadowShapes/ShadowTricycle.ShadowTricycle_C|GetModel _asshadow_tricycle)))
                                                                (:CastFailed
                                                                  (bind _asshadow_turtle (Utilities|Casting|CastToShadowTurtle (LocalVariables|GetInput))
                                                                    (:then
                                                                      (return (Variables|/Game/Blueprints/ShadowShapes/ShadowTurtle.ShadowTurtle_C|GetModel _asshadow_turtle)))
                                                                    (:CastFailed
                                                                      (bind _asshadow_unicycle (Utilities|Casting|CastToShadowUnicycle (LocalVariables|GetInput))
                                                                        (:then
                                                                          (return (Variables|/Game/Blueprints/ShadowShapes/ShadowUnicycle.ShadowUnicycle_C|GetModel _asshadow_unicycle)))
                                                                        (:CastFailed
                                                                          (bind _asshadow_wheelchair (Utilities|Casting|CastToShadowWheelchair (LocalVariables|GetInput))
                                                                            (:then
                                                                              (return (Variables|/Game/Blueprints/ShadowShapes/ShadowWheelchair.ShadowWheelchair_C|GetModel _asshadow_wheelchair)))
                                                                            (:CastFailed
                                                                              (bind _asshadow_wind_turbine (Utilities|Casting|CastToShadowWindTurbine (LocalVariables|GetInput)))
                                                                              (return (Variables|/Game/Blueprints/ShadowShapes/ShadowWindTurbine.ShadowWindTurbine_C|GetModel _asshadow_wind_turbine)))))))))))))))))))))))))))))))))))))))))

(fn CompareShadowSize
  (params (Actor%20A :type Actor%20Object%20Reference) (Actor%20B :type Actor%20Object%20Reference))
  (return (< (Math|Float|Absolute(Float) (- (/ (Math|Vector|Distance(Vector) (Transformation|GetActorLocation Actor%20A) "0, 0,150.000000") (Math|Vector|Distance(Vector) (Transformation|GetActorLocation Actor%20B) "0, 0,150.000000")) (/ (.x (Transformation|GetActorScale3D Actor%20B)) (.x (Transformation|GetActorScale3D Actor%20A))))) (Variables|Default|GetShadow%20Size%20Similarity%20Threshold))))

(fn UpdatePlayerShadows
  (for (_array_element _array_index) (Variables|/Game/Blueprints/PlayerManager.PlayerManager_C|GetplayerPairs (Variables|Default|GetPlayerManager))
    (LocalVariables|SetIndex _array_index)
    (bind _model (CallFunction|GetModel (.playershadow (Utilities|Array|Get(acopy) (Variables|Default|GetShadow%20Pairs) (LocalVariables|GetIndex)))))
    (bind _yaw (CallFunction|GetPitchandYaw (.playerdirection (Utilities|Array|Get(acopy) (Variables|Default|GetShadow%20Pairs) (LocalVariables|GetIndex))) (Variables|/Game/Blueprints/PlayerPair.PlayerPair_C|GetTrackerR _array_element))) ; Something's broken here
    (Transformation|SetRelativeRotation _model (Math|Rotator|MakeRotator (.roll (Variables|/Script/Engine.SceneComponent|GetRelativeRotation _model)) (.pitch (Variables|/Script/Engine.SceneComponent|GetRelativeRotation _model)) _yaw) false false)
    ;[1 1 1] Distance Method (half - tested but hopefully not broken)
    (bind _location (CallFunction|GetSpawnLocation (.playerangle (Utilities|Array|Get(acopy) (Variables|Default|GetShadow%20Pairs) (LocalVariables|GetIndex))) (Math|Float|Clamp(Float) (Math|Vector|Distance(Vector) (Transformation|GetActorLocation (Variables|/Game/Blueprints/PlayerPair.PlayerPair_C|GetTrackerR _array_element)) "0, 0, 0") (Variables|Default|GetMinimum%20Spawn%20Distance) (Variables|Default|GetMaximum%20Spawn%20Distance))))
    (Transformation|SetActorLocation (.playershadow (Utilities|Array|Get(acopy) (Variables|Default|GetShadow%20Pairs) (LocalVariables|GetIndex))) _location false false)))

(fn GetDirectionfromAngle
  (params (Angle :type Float%20%28single-precision%29))
  (if (Math|Float|InRange(Float) Angle 45.0 135.0 false)
    (return "NewEnumerator2")
    (elif (Math|Float|InRange(Float) Angle 135.0 225.0 false)
      (return "NewEnumerator1")
      (elif (Math|Float|InRange(Float) Angle 225.0 315.0 false)
        (return "NewEnumerator3")
        (else
          (return "NewEnumerator0"))))))

(fn GetPitchandYaw
  (params (Direction :type Direction%20Enum :default "NewEnumerator0") (DA%20Tracker :type Actor%20Object%20Reference))
  (bind _yaw_window_size (Variables|Default|GetYaw%20Window%20Size))
  (bind _yaw_window_size_2 (Variables|Default|GetYaw%20Window%20Size))
  (bind _yaw_window_size_3 (Variables|Default|GetYaw%20Window%20Size))
  (bind _yaw_window_size_4 (Variables|Default|GetYaw%20Window%20Size))
  (LocalVariables|SetTracker%20Location (Transformation|GetActorLocation DA%20Tracker))
  (switch Utilities|FlowControl|Switch|SwitchonDirection Direction
    (:NewEnumerator0
      (LocalVariables|SetYaw%20Output (* (/ (+ (/ _yaw_window_size 2.0) (.y (LocalVariables|GetTracker%20Location))) _yaw_window_size) 3.6e+02)))
    (:NewEnumerator1
      (LocalVariables|SetYaw%20Output (* (/ (- (/ _yaw_window_size_2 2.0) (.y (LocalVariables|GetTracker%20Location))) _yaw_window_size_2) 3.6e+02)))
    (:NewEnumerator2
      (LocalVariables|SetYaw%20Output (* (/ (+ (/ _yaw_window_size_3 2.0) (.x (LocalVariables|GetTracker%20Location))) _yaw_window_size_3) 3.6e+02)))
    (:NewEnumerator3
      (LocalVariables|SetYaw%20Output (* (/ (- (/ _yaw_window_size_4 2.0) (.x (LocalVariables|GetTracker%20Location))) _yaw_window_size_4) 3.6e+02))))
  (return (LocalVariables|GetYaw%20Output)))

(fn SpawnProxyShadow
  (params (Shadow%20Parameters :type Map%20of%20Strings%20to%20Strings) (Target%20Shadow :type Boolean))
  (bind _value (Utilities|Map|Find Shadow%20Parameters "Index"))
  (bind _number_of_players (Variables|Default|GetNumber%20of%20Players))
  (bind _shadow_pairs (Variables|Default|GetShadow%20Pairs))
  (bind _returnvalue (Math|Conversions|ToInteger(Byte) _value))
  (bind _returnvalue_2 (Math|Conversions|ToFloat(Integer) _number_of_players))
  (bind _output (Utilities|Array|Get(acopy) _shadow_pairs _returnvalue))
  (bind _output_get (LocalVariables|SetAngle (* (Math|Conversions|ToFloat(Integer) (.Value (Utilities|Map|Find Shadow%20Parameters "Player"))) (/ 3.6e+02 (Math|Conversions|ToFloat(Integer) (Variables|Default|GetNumber%20of%20Players))))))
  (bind _location (CallFunction|GetSpawnLocation _output_get (Math|Conversions|ToFloat(Integer) (.Value (Utilities|Map|Find Shadow%20Parameters "Distance")))))
  (bind (_shadow _pitch_output _roll_output) (CallFunction|SpawnSingleShadow (Utilities|Array|Get(acopy) (Variables|Default|GetShadow%20Classes) (Math|Conversions|ToInteger(Byte) (.Value (Utilities|Map|Find Shadow%20Parameters "Shadow")))) _location (LocalVariables|GetAngle) (Math|Conversions|ToFloat(Integer) (.Value (Utilities|Map|Find Shadow%20Parameters "Pitch"))) (Math|Conversions|ToFloat(Integer) (.Value (Utilities|Map|Find Shadow%20Parameters "Roll"))) (Math|Conversions|ToFloat(Integer) (.Value (Utilities|Map|Find Shadow%20Parameters "Yaw"))) false))
  (bind _direction (CallFunction|GetDirectionfromAngle (LocalVariables|GetAngle)))
  (if Target%20Shadow
    (Utilities|Array|SetArrayElem (Variables|Default|GetShadow%20Pairs) (Math|Conversions|ToInteger(Byte) (.Value (Utilities|Map|Find Shadow%20Parameters "Index"))) (Utilities|Struct|MakeShadowPair _shadow 0 "(ShadowClass_2_C4BB407C49D8927D41A62C95D03827D2=None,MinimumScale_8_9331718C4F685E0DBA09F39FC278B456=0.000000,MaximumScale_9_9646880743E7E3E564982FA0AAEF93B7=0.000000)" (LocalVariables|GetAngle) 0.0 _direction _pitch_output _roll_output) true)
    (else
      (Utilities|Array|SetArrayElem (Variables|Default|GetShadow%20Pairs) _returnvalue (Utilities|Struct|MakeShadowPair (.playershadow _output) _shadow (.sourceclass _output) (.playerangle _output) (+ (* (Math|Conversions|ToFloat(Integer) (.Value (Utilities|Map|Find Shadow%20Parameters "Index"))) (/ 3.6e+02 _returnvalue_2)) (/ 1.8e+02 _returnvalue_2)) (.playerdirection _output) (.pitch _output) (.roll _output))))))