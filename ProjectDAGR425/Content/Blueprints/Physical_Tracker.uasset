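; Physical_Tracker is an actor that mirrors the location and orientation of a referenced DATracker while CopyDATracker is enabled.
; Each tick it takes the tracker's location in DA space and applies it directly as the actor location.
; It combines the relative rotation with RotationOffset, scales the resulting forward vector by RotationMultiplier, then rebuilds rotation from that vector, which discards roll.
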(event EventBeginPlay)

(event Collision|EventActorBeginOverlap
  (params (OtherActor :type Actor%20Object%20Reference)))

(event EventTick
  (params (DeltaSeconds :type Float%20%28single-precision%29))
  (bind _da_tracker (Variables|Default|GetDA%20Tracker))
  (bind _rotationoffset (Variables|Default|GetRotationOffset))
  (bind (_x _y _z) (Math|Vector|BreakVector _rotationoffset))
  (if (Variables|Default|GetcopyDATracker)
    (bind _location (Default|GetLocationinDA _da_tracker))
    (bind _rotation (Default|GetRelativeRotation _da_tracker))
    (Transformation|SetActorLocationAndRotation _location (Math|Conversions|RotationFromXVector (* (Math|Rotator|GetRotationXVector (Math|Rotator|CombineRotators _rotation (Math|Rotator|MakeRotator _x _y _z))) (Variables|Default|GetRotationMultiplier))))))

(fn ConstructionScript)