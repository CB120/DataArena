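; PlayerPair represents one player as a numbered pair of right and left trackers, assigned through AssignTrackersAndNumber.
; Query functions return each tracker's pose, plus the distance, vector, height difference and forward-vector dot product between the two.
; It also exposes the DATracker of Physical_Tracker actors and a colour looked up by player number, with a leftover debug print.
; Event graph logic is empty, and the RotatorInvert adjustment mentioned in comments is not applied.
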(event EventBeginPlay)

(event Collision|EventActorBeginOverlap
  (params (OtherActor :type Actor%20Object%20Reference)))

(event EventTick
  (params (DeltaSeconds :type Float%20%28single-precision%29)))

(fn ConstructionScript)

(fn AssignTrackersandNumber
  (params (trackerR :type Actor%20Object%20Reference) (trackerL :type Actor%20Object%20Reference) (playerNumber :type Integer))
  (Variables|Default|SetTrackerR trackerR)
  (Variables|Default|SetTrackerL trackerL)
  (Variables|Default|SetplayerNumber playerNumber))

(fn GetTrackerForwardVector
  (params (trackerType :type ETrackerType%20Enum :default "NewEnumerator0"))
  ;[1 1 1] This function returns the specified tracker's forward vector - modified by RotatorInvert
  (switch Utilities|FlowControl|Switch|SwitchonETrackerType trackerType
    (:NewEnumerator0
      (return (Math|Vector|GetForwardVector (Transformation|GetWorldRotation (Variables|/Script/Engine.Actor|GetRootComponent (Variables|Default|GetTrackerR))))))
    (:NewEnumerator1
      (return (Math|Vector|GetForwardVector (Transformation|GetWorldRotation (Variables|/Script/Engine.Actor|GetRootComponent (Variables|Default|GetTrackerL))))))))

(fn GetTrackerRotator
  (params (trackerType :type ETrackerType%20Enum :default "NewEnumerator0"))
  (bind _trackerr (Variables|Default|GetTrackerR))
  (bind _trackerl (Variables|Default|GetTrackerL))
  (bind _returnvalue (Transformation|GetActorRotation _trackerr))
  (bind _returnvalue_2 (Transformation|GetActorRotation _trackerl))
  (bind (_roll _pitch _yaw) (Math|Rotator|BreakRotator _returnvalue_2))
  (bind (_roll_2 _pitch_2 _yaw_2) (Math|Rotator|BreakRotator _returnvalue))
  (bind _returnvalue_3 (Math|Vector|MakeVector _roll_2 _pitch_2 _yaw_2))
  (bind _returnvalue_4 (Math|Vector|MakeVector _roll _pitch _yaw))
  (bind (_x _y _z) (Math|Vector|BreakVector _returnvalue_4))
  (bind (_x_2 _y_2 _z_2) (Math|Vector|BreakVector _returnvalue_3))
  ;[1 1 1] This function returns the specified tracker's rotator - modified by RotatorInvert (I DON'T ACTUALLY KNOW IF THIS WORKS, UHHH)
  (switch Utilities|FlowControl|Switch|SwitchonETrackerType trackerType
    (:NewEnumerator0
      (return (Math|Rotator|MakeRotator _x_2 _y_2 _z_2)))
    (:NewEnumerator1
      (return (Math|Rotator|MakeRotator _x _y _z)))))

(fn GetTrackerLocation
  (params (trackerType :type ETrackerType%20Enum :default "NewEnumerator0"))
  (switch Utilities|FlowControl|Switch|SwitchonETrackerType trackerType
    (:NewEnumerator0
      (return (Transformation|GetActorLocation (Variables|Default|GetTrackerR))))
    (:NewEnumerator1
      (return (Transformation|GetActorLocation (Variables|Default|GetTrackerL))))))

(fn GetDistanceBetweenTrackers
  (return (Math|Float|Absolute(Float) (Math|Vector|VectorLength (- (Transformation|GetWorldLocation (Variables|/Script/Engine.Actor|GetRootComponent (Variables|Default|GetTrackerL))) (Transformation|GetWorldLocation (Variables|/Script/Engine.Actor|GetRootComponent (Variables|Default|GetTrackerR))))))))

(fn GetVectorBetweenTrackers
  (params (pointingFrom :type ETrackerType%20Enum :default "NewEnumerator0") (isNormalised :type Boolean))
  ;[1 1 1] This function returns the vector pointing from the specified tracker to the other tracker (optionally normalised)
  ;[1 1 1] L to R
  (bind _location (CallFunction|GetTrackerLocation "NewEnumerator0"))
  (bind _location_2 (CallFunction|GetTrackerLocation "NewEnumerator1"))
  (switch Utilities|FlowControl|Switch|SwitchonETrackerType pointingFrom
    (:NewEnumerator0
      (if isNormalised
        (return (Math|Vector|Normalize (* (- _location _location_2) -1.0)))
        (else
          (return (* (- _location _location_2) -1.0)))))
    (:NewEnumerator1
      (if isNormalised
        (return (Math|Vector|Normalize (- _location _location_2)))
        (else
          (return (- _location _location_2)))))))

(fn GetTrackerasDATracker
  (params (trackerType :type ETrackerType%20Enum :default "NewEnumerator0"))
  (switch Utilities|FlowControl|Switch|SwitchonETrackerType trackerType
    (:NewEnumerator0
      (bind _asphysical_tracker (Utilities|Casting|CastToPhysical_Tracker (Variables|Default|GetTrackerR)))
      (return (Variables|/Game/Blueprints/Physical_Tracker.Physical_Tracker_C|GetDA%20Tracker _asphysical_tracker) true))
    (:NewEnumerator1
      (bind _asphysical_tracker_2 (Utilities|Casting|CastToPhysical_Tracker (Variables|Default|GetTrackerL)))
      (return (Variables|/Game/Blueprints/Physical_Tracker.Physical_Tracker_C|GetDA%20Tracker _asphysical_tracker_2) true))))

(fn GetDotProductOfTrackerForwardVectors
  (bind _forwardvector (CallFunction|GetTrackerForwardVector "NewEnumerator0"))
  (bind _forwardvector_2 (CallFunction|GetTrackerForwardVector "NewEnumerator1"))
  (return (Math|Vector|DotProduct _forwardvector _forwardvector_2)))

(fn GetHeightBetweenTrackers
  (bind _location (CallFunction|GetTrackerLocation "NewEnumerator0"))
  (bind _location_2 (CallFunction|GetTrackerLocation "NewEnumerator1"))
  (return (- (.z _location) (.z _location_2))))

(fn GetPlayerColor
  (bind _playernumber (Variables|Default|GetplayerNumber))
  (Development|PrintString (Utilities|String|ToString(Integer) _playernumber) true true "(R=1.000000,G=0.042958,B=0.000000,A=1.000000)")
  (return (Math|Conversions|ToLinearColor(Color) (Utilities|Array|Get(acopy) (Variables|Default|GetplayerColours) _playernumber))))